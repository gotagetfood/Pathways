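; A possessable color-line brick pawn that marks its possession state through the Cube's custom depth stencil value.
; Possession switches the stencil value, and unpossession or the Interact input switches it back.
; Interact also hands player control back to the first-person character.
; On BeginPlay it moves its Camera to that character's camera transform, then runs the parent BeginPlay.
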(event `self.ReceiveUnpossessed`
  (params (OldController :type "Controller Object Reference"))
  (`PrimitiveComponent.SetCustomDepthStencilValue` (`self.Cube`) 1))

(event `EnhancedInput|/Game/FirstPerson/Input/Actions/IA_Interact`
  (params (ActionValue :type Boolean) (ElapsedSeconds :type "Float (double-precision)") (TriggeredSeconds :type "Float (double-precision)") (InputAction :type "InputAction Object Reference" :default "/Game/FirstPerson/Input/Actions/IA_Interact.IA_Interact"))
  (:`Started`
    (`PrimitiveComponent.SetCustomDepthStencilValue` (`self.Cube`) 1)
    (bind _returnvalue (`GameplayStatics.GetActorOfClass` "/Game/FirstPerson/Blueprints/BP_FirstPersonCharacter.BP_FirstPersonCharacter_C"))
    (`Controller.Possess` (`GameplayStatics.GetPlayerController` 0) _returnvalue)))

(event `self.ReceivePossessed`
  (params (NewController :type "Controller Object Reference"))
  (`PrimitiveComponent.SetCustomDepthStencilValue` (`self.Cube`) 2))

(event `self.ReceiveBeginPlay`
  (bind _returnvalue (`GameplayStatics.GetActorOfClass` "/Game/FirstPerson/Blueprints/BP_FirstPersonCharacter.BP_FirstPersonCharacter_C"))
  (bind _camera_transform (`/Game/FirstPerson/Blueprints/BP_FirstPersonCharacter.get Camera Transform` _returnvalue))
  (`SceneComponent.K2_SetWorldTransform` (`self.Camera`) _camera_transform false false)
  (`parent.ReceiveBeginPlay`))

(fn `UserConstructionScript`)