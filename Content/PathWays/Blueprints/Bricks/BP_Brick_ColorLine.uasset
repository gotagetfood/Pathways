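; Possessable color-line puzzle brick that steps across a grid, painting back-board cells with its material and light color.
; Move input offsets the grid index by one or a row; walls and color lines block, while timelines animate paint and movement.
; Back cells come from the puzzle podium, and the camera copies the first-person view at start.
; Interact repossesses the first-person character; undo and reset inputs are empty, and switch is unfinished.
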(event `EnhancedInput|/Game/FirstPerson/Input/Actions/IA_Move`
  (params (ActionValue :type "Vector2D Structure") (ElapsedSeconds :type "Float (double-precision)") (TriggeredSeconds :type "Float (double-precision)") (InputAction :type "InputAction Object Reference" :default "/Game/FirstPerson/Input/Actions/IA_Move.IA_Move"))
  (bind _current_index (`self.Current Index`))
  (bind _output (`|GetArrayItem` (`self.Spawned Cubes (back)`) (`self.Current Index`)))
  (bind _returnvalue (+ (`self.Current Index`) -1))
  (bind _returnvalue_2 (+ (`self.Current Index`) 1))
  (bind _returnvalue_3 (- (`self.Current Index`) (`self.Columns`)))
  (bind _returnvalue_4 (+ (`self.Current Index`) (`self.Columns`)))
  (bind _cube (`/Game/PathWays/Blueprints/Bricks/BP_Brick_ABase.Cube` _output))
  ;[1 1 1] Puzzle Movement
  (:`Started`
    (if (not (`self.InMovement`))
      (set `self.InMovement` true)
      (set `self.Wall Index` _current_index)
      (set `self.Current Location` (`|GetArrayItem` (`self.Movement Locations`) _current_index))
      (if (== (1.0 0.0) ActionValue)
        (set `self.Moveing Location` (`|GetArrayItem` (`self.Movement Locations`) _returnvalue_2))
        (set `self.Current Index` _returnvalue_2)
        (switch `/Game/PathWays/Blueprints/E_BrickType` (`/Game/PathWays/Blueprints/Bricks/BP_Brick_ABase.BrickType` (`|GetArrayItem` (`self.Spawned Cubes (back)`) (`self.Current Index`))) :!label _label
          (:`NewEnumerator0`
            (set `self.Current Index` (`self.Wall Index`) :!label _label_2)
            (set `self.InMovement` false))
          (:`NewEnumerator1`
            (goto _label_2))
          (:`NewEnumerator2`
            (`PrimitiveComponent.SetMaterial` _cube 0 (`self.BB Matreal`))
            (bind (_direction _magic_carpet_line) (`Timeline|Timeline_1` :!via `PlayFromStart`)
              (:`Update`
                (`MeshComponent.SetScalarParameterValueOnMaterials` _cube "Percentage" _magic_carpet_line))
              (:`Finished`
                (`LightComponent.SetLightColor` (`/Game/PathWays/Blueprints/Bricks/BP_Brick_ABase.SpotLight` _output) (`self.BB Light Color`) true)
                (set `self.End Transfom` (`self.Moveing Location`) :!label _label_3)
                (bind (_direction_2 _magic_carpet_line_2) (`Timeline|Timeline_0` :!via `PlayFromStart`)
                  (:`Update`
                    (`SceneComponent.K2_SetWorldTransform` (`self.Cube`) (`KismetMathLibrary.TLerp` (`self.Current Location`) (`self.Moveing Location`) _magic_carpet_line_2) false false))
                  (:`Finished`
                    (set `self.InMovement` false))))))
          (:`NewEnumerator3`
            (goto _label_3)))
        (elif (== (-1.0 0.0) ActionValue)
          (set `self.Moveing Location` (`|GetArrayItem` (`self.Movement Locations`) _returnvalue))
          (set `self.Current Index` _returnvalue)
          (goto _label)
          (elif (== (0.0 1.0) ActionValue)
            (set `self.Moveing Location` (`|GetArrayItem` (`self.Movement Locations`) _returnvalue_3))
            (set `self.Current Index` _returnvalue_3)
            (goto _label)
            (elif (== (0.0 -1.0) ActionValue)
              (set `self.Moveing Location` (`|GetArrayItem` (`self.Movement Locations`) _returnvalue_4))
              (set `self.Current Index` _returnvalue_4)
              (goto _label))))))))

(event `EnhancedInput|/Game/FirstPerson/Input/Actions/IA_Undo`
  (params (ActionValue :type Boolean) (ElapsedSeconds :type "Float (double-precision)") (TriggeredSeconds :type "Float (double-precision)") (InputAction :type "InputAction Object Reference" :default "/Game/FirstPerson/Input/Actions/IA_Undo.IA_Undo"))
  ;[1 1 1] Puzzle Movement
)

(event `EnhancedInput|/Game/FirstPerson/Input/Actions/IA_Reset`
  (params (ActionValue :type Boolean) (ElapsedSeconds :type "Float (double-precision)") (TriggeredSeconds :type "Float (double-precision)") (InputAction :type "InputAction Object Reference" :default "/Game/FirstPerson/Input/Actions/IA_Reset.IA_Reset"))
  ;[1 1 1] Puzzle Movement
)

(event `EnhancedInput|/Game/FirstPerson/Input/Actions/IA_CLReset`
  (params (ActionValue :type Boolean) (ElapsedSeconds :type "Float (double-precision)") (TriggeredSeconds :type "Float (double-precision)") (InputAction :type "InputAction Object Reference" :default "/Game/FirstPerson/Input/Actions/IA_CLReset.IA_CLReset"))
  ;[1 1 1] Puzzle Movement
)

(event `EnhancedInput|/Game/FirstPerson/Input/Actions/IA_Switch`
  (params (ActionValue :type Boolean) (ElapsedSeconds :type "Float (double-precision)") (TriggeredSeconds :type "Float (double-precision)") (InputAction :type "InputAction Object Reference" :default "/Game/FirstPerson/Input/Actions/IA_Switch.IA_Switch"))
  ;[1 1 1] Puzzle Movement
  (:`Triggered`
    (`GameplayStatics.GetAllActorsOfClass` "BP_Brick_ColorLine_C")))

(event `EnhancedInput|/Game/FirstPerson/Input/Actions/IA_Interact`
  (params (ActionValue :type Boolean) (ElapsedSeconds :type "Float (double-precision)") (TriggeredSeconds :type "Float (double-precision)") (InputAction :type "InputAction Object Reference" :default "/Game/FirstPerson/Input/Actions/IA_Interact.IA_Interact"))
  ;[1 1 1] Possession
  (:`Started`
    (`PrimitiveComponent.SetCustomDepthStencilValue` (`self.Cube`) 1)
    (bind _returnvalue (`GameplayStatics.GetActorOfClass` "/Game/FirstPerson/Blueprints/BP_FirstPersonCharacter.BP_FirstPersonCharacter_C"))
    (`Controller.Possess` (`GameplayStatics.GetPlayerController` 0) _returnvalue)))

(event `self.ReceivePossessed`
  (params (NewController :type "Controller Object Reference"))
  ;[1 1 1] Possession
  (`PrimitiveComponent.SetCustomDepthStencilValue` (`self.Cube`) 2))

(event `self.ReceiveUnpossessed`
  (params (OldController :type "Controller Object Reference"))
  ;[1 1 1] Possession
  (`PrimitiveComponent.SetCustomDepthStencilValue` (`self.Cube`) 1))

(event `self.ReceiveBeginPlay`
  ;[1 1 1] Begin Play
  (`self.DisableInput` null)
  (`|ExecutionSequence`
    (:`then_0`
      (bind _returnvalue (`GameplayStatics.GetActorOfClass` "/Game/FirstPerson/Blueprints/BP_FirstPersonCharacter.BP_FirstPersonCharacter_C"))
      (bind _camera_transform (`/Game/FirstPerson/Blueprints/BP_FirstPersonCharacter.get Camera Transform` _returnvalue))
      (`SceneComponent.K2_SetWorldTransform` (`self.Camera`) _camera_transform false false)
      (`parent.ReceiveBeginPlay`))
    (:`then_1`
      (`KismetSystemLibrary.Delay` 0.1)
      (bind _output_get (set `self.Spawned Cubes (back)` (`/Game/PathWays/Blueprints/BP_Puzzle_Podium.Spawned Cube Stuff Back` (`self.Puzzle Podium Ref`))))
      (bind _output (`|GetArrayItem` _output_get (`self.Current Index`)))
      (bind _cube (`/Game/PathWays/Blueprints/Bricks/BP_Brick_ABase.Cube` _output))
      (`PrimitiveComponent.SetMaterial` _cube 0 (`self.BB Matreal`))
      (bind (_direction _magic_carpet_line) (`Timeline|Timeline_2` :!via `PlayFromStart`)
        (:`Update`
          (`MeshComponent.SetScalarParameterValueOnMaterials` _cube "Percentage" _magic_carpet_line))
        (:`Finished`
          (`LightComponent.SetLightColor` (`/Game/PathWays/Blueprints/Bricks/BP_Brick_ABase.SpotLight` _output) (`self.BB Light Color`) true))))
    (:`then_2`
      (`KismetSystemLibrary.Delay` 2.5)
      (`self.EnableInput` null))))

(fn `UserConstructionScript`)