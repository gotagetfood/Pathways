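; BP_Brick_ABase is a brick actor for PathWays that animates itself in on spawn and out on destruction.
; On BeginPlay a timeline, started at a random offset, lerps the cube from the root transform to EndTransfom, then calls SetLight, which is empty here.
; DestroyBrick removes the spotlight, then a second timeline shrinks the cube to zero scale with a random rotation before destroying the actor.
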(event `self.ReceiveBeginPlay`
  (set `self.Start Transform` (`SceneComponent.K2_GetComponentToWorld` (`self.DefaultSceneRoot`)))
  (`|ExecutionSequence`
    (:`then_0`
      (bind (_direction _magic_carpet_line) (`Timeline|Spawning Timeline` :`NewTime` (`KismetMathLibrary.RandomFloatInRange` 0.0 0.5) :!via `SetNewTime` :!label _label)
        (:`Update`
          (`SceneComponent.K2_SetWorldTransform` (`self.Cube`) (`KismetMathLibrary.TLerp` (`self.Start Transform`) (`self.End Transfom`) _magic_carpet_line) false false))
        (:`Finished`
          (`self.set Light`))))
    (:`then_1`
      (goto _label))))

(event `Destroy Brick`
  (`self.Turn Off Light`)
  (set `self.Start Transform` (`SceneComponent.K2_GetComponentToWorld` (`self.Cube`)))
  (set `self.End Transfom` (`KismetMathLibrary.MakeTransform` (.location (`self.End Transfom`)) (`KismetMathLibrary.RandomRotator` false) (0.0 0.0 0.0)))
  (bind (_direction _magic_carpet_line) (`Timeline|Timeline`)
    (:`Update`
      (`SceneComponent.K2_SetWorldTransform` (`self.Cube`) (`KismetMathLibrary.TLerp` (`self.Start Transform`) (`self.End Transfom`) _magic_carpet_line) false false))
    (:`Finished`
      (`self.K2_DestroyActor`))))

(event `Turn Off Light`
  (`ActorComponent.K2_DestroyComponent` (`self.SpotLight`)))

(fn `set Light`)

(fn `UserConstructionScript`)