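; BP_fence_gate is a fence gate that opens when its count of active power connections equals the required number.
; Poweron and PowerOff adjust the count, then rerun the open/close animation on every change.
; Two timelines lerp FencesPolls1's relative rotation between closed and open, with the open rotation built from Rotation at BeginPlay.
; Opening also adds an audio component, and closing restarts from the open rotation.
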(event `/Game/PathWays/Blueprints/interfaces/IN_Power.PowerOn`
  (bind _number_of_active_conections (`self.Number Of Active Conections`))
  (`KismetSystemLibrary.PrintString` "on")
  (`/Engine/EditorBlueprintResources/StandardMacros.IncrementInt` _number_of_active_conections
    (:`  `
      (if (== _number_of_active_conections (`self.Number Of Conections`)) :!label _label
        (`KismetSystemLibrary.PrintString` "OPEN")
        (set `self.Open` true)
        (else
          (`KismetSystemLibrary.PrintString` "CLOSE")
          (set `self.Open` false)))
      (`self.Open | Close`))))

(event `/Game/PathWays/Blueprints/interfaces/IN_Power.PowerOff`
  (`KismetSystemLibrary.PrintString` "off")
  (`/Engine/EditorBlueprintResources/StandardMacros.DecrementInt` (`self.Number Of Active Conections`)
    (:`  `
      (goto _label))))

(event `self.ReceiveBeginPlay`
  (set `self.Open Rotation` (`KismetMathLibrary.MakeRotator` 0.0 0.0 (`self.Rotation`))))

(event `Open | Close`
  (if (`self.Open`)
    (`AddComponent|NODE_AddAudioComponent-0`)
    ;[0.2934 1 0.1701] Open
    (bind (_direction _gate) (`Timeline|Timeline` :!via `PlayFromStart`)
      (:`Update`
        (`SceneComponent.K2_SetRelativeRotation` (`self.Fences Polls1`) (`KismetMathLibrary.RLerp` (`self.Closed Rotation`) (`self.Open Rotation`) _gate true) false false)))
    (else
      ;[1 0.1631 0.08678] Close
      (bind (_direction_2 _gate_2) (`Timeline|Timeline_0` :!via `PlayFromStart`)
        (:`Update`
          (`SceneComponent.K2_SetRelativeRotation` (`self.Fences Polls1`) (`KismetMathLibrary.RLerp` (`self.Open Rotation`) (`self.Closed Rotation`) _gate_2 true) false false))))))

(fn `UserConstructionScript`)