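; Puzzle podium actor that launches a color-line grid puzzle and feeds its solved state into a linked cable.
; Interacting reads the puzzle by ID, spawns bricks on a two-layer grid fitted to the cell size and possesses a color-line brick.
; Interacting while in the puzzle toggles Solved/Unsolved and the cable.
; Power events restore the saved state, and three spinning meshes are recolored per state through dynamic materials.
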(event `/Game/PathWays/Blueprints/interfaces/IN_Power.PowerOn`
  (bind _linked_cable (`self.Linked Cable`))
  ;[1 1 1] State Switching
  (`KismetSystemLibrary.PrintString` "on")
  (set `self.State` (`self.State_Past`))
  (switch `/Game/PathWays/Blueprints/E_Podium_State` (`self.State`) :!label _label
    (:`NewEnumerator0`
      (`/Engine/EditorBlueprintResources/StandardMacros.IsValid` _linked_cable
        (:`Is Valid`
          (set `/Game/PathWays/Blueprints/BP_Cable.isFilling` false _linked_cable :!label _label_2)
          (`/Game/PathWays/Blueprints/BP_Cable.Unactivate Next` _linked_cable))
        (:`Is Not Valid`
          (`KismetSystemLibrary.PrintString` "no Cable END" :!label _label_3))))
    (:`NewEnumerator1`
      (`/Engine/EditorBlueprintResources/StandardMacros.IsValid` _linked_cable
        (:`Is Valid`
          (goto _label_2))
        (:`Is Not Valid`
          (goto _label_3))))
    (:`NewEnumerator2`
      (`/Engine/EditorBlueprintResources/StandardMacros.IsValid` _linked_cable
        (:`Is Valid`
          (set `/Game/PathWays/Blueprints/BP_Cable.isFilling` true _linked_cable)
          (`/Game/PathWays/Blueprints/BP_Cable.Activate Next` _linked_cable))
        (:`Is Not Valid`
          (goto _label_3)))))
  (`self.UpdateState`))

(event `Exit Puzzle`
  (bind _spawned_cube_stuff (`self.Spawned Cube Stuff`))
  ;[1 1 1] Delete Cubes
  (for _ _spawned_cube_stuff
    (`/Game/PathWays/Blueprints/Bricks/BP_ABaseBrick.Destroy Brick` _spawned_cube_stuff))
  (`KismetArrayLibrary.Array_Clear` _spawned_cube_stuff))

(event `/Game/PathWays/Blueprints/interfaces/IN_Power.PowerOff`
  ;[1 1 1] State Switching
  (`KismetSystemLibrary.PrintString` "off")
  (set `self.State` (`self.State_Past`))
  (goto _label))

(event `Set State`
  (params (State :type "/Game/PathWays/Blueprints/E_Podium_State Enum" :default "NewEnumerator0"))
  ;[1 1 1] State Switching
  (set `self.State_Past` State))

(event `/Game/PathWays/Blueprints/interfaces/IN_Interact.Interacted`
  (params (`Spawn Location` :type "Transform Structure"))
  (bind _spawn_location_center (`self.Spawn Location Center`))
  (bind _scaler (`self.Scaler`))
  (bind _linked_cable (`self.Linked Cable`))
  (bind (_returnvalue_x _returnvalue_y _returnvalue_z) (`KismetMathLibrary.BreakVector` (`KismetMathLibrary.TransformLocation` _spawn_location_center)))
  (bind _returnvalue (`KismetMathLibrary.TransformRotation` _spawn_location_center))
  (bind _returnvalue_2 (`KismetMathLibrary.TransformLocation` _spawn_location_center))
  (bind _returnvalue_x_2 (`KismetMathLibrary.BreakVector` (`KismetMathLibrary.TransformLocation` _spawn_location_center)))
  (bind _returnvalue_3 (`KismetMathLibrary.FMin` (`self.Puzzle Width`) (`self.Puzzle Height`)))
  (bind _returnvalue_4 (* (`self.Cube Spaceing`) _returnvalue_3))
  (bind _returnvalue_5 (`KismetMathLibrary.Conv_DoubleToVector` (* 0.2 _returnvalue_3)))
  (bind _returnvalue_6 (/ _returnvalue_4 2.0))
  (if (`self.InPuzzle`)
    (set `self.InPuzzle` false)
    ;[1 1 1] State Switching
    (switch `/Game/PathWays/Blueprints/E_Podium_State` (`self.State`)
      (:`NewEnumerator1`
        (set `self.State` "NewEnumerator2")
        (`/Engine/EditorBlueprintResources/StandardMacros.IsValid` _linked_cable
          (:`Is Valid`
            (set `/Game/PathWays/Blueprints/BP_Cable.isFilling` true _linked_cable)
            (`/Game/PathWays/Blueprints/BP_Cable.Activate Next` _linked_cable))
          (:`Is Not Valid`
            (`KismetSystemLibrary.PrintString` "no Cable" :!label _label_4))))
      (:`NewEnumerator2`
        (set `self.State` "NewEnumerator1")
        (`/Engine/EditorBlueprintResources/StandardMacros.IsValid` _linked_cable
          (:`Is Valid`
            (set `/Game/PathWays/Blueprints/BP_Cable.isFilling` false _linked_cable)
            (`/Game/PathWays/Blueprints/BP_Cable.Unactivate Next` _linked_cable))
          (:`Is Not Valid`
            (goto _label_4)))))
    (`self.UpdateState`)
    (else
      (bind _outactors (`GameplayStatics.GetAllActorsOfClass` "/Game/PathWays/Blueprints/Bricks/BP_ColorLine_Brick.BP_ColorLine_Brick_C"))
      (if (`KismetArrayLibrary.Array_IsEmpty` _outactors)
        (switch `/Game/PathWays/Blueprints/E_Podium_State` (`self.State`)
          (:`NewEnumerator1`
            _)
          (:`NewEnumerator2`
            _))
        (set `self.Spawn Location Center` `Spawn Location`)
        (set `self.InPuzzle` true)
        (bind (_outrows _outcolumns _returnvalue_7) (`PuzzleReader.ReadPuzzle` (`self.Puzzle Reader`) (`self.Puzzle ID`)))
        (set `self.Rows` _outrows)
        (set `self.Columns` _outcolumns)
        (set `self.Grid Objects` _returnvalue_7)
        (`KismetArrayLibrary.Array_Clear` (`self.Grid Locations`))
        (set `self.Puzzle Height` (/ (`self.CellSize`) (`self.Rows`)))
        (`KismetArrayLibrary.Array_Clear` (`self.Grid Locations Forward`))
        (set `self.Puzzle Width` (/ (`self.CellSize`) (`self.Columns`)))
        ;[1 1 1] Generate Grid Locations
        (set `self.Scaler` _returnvalue_4)
        (set `self.Offset Y` (- (/ (* (`self.Columns`) _returnvalue_4) -2.0) _returnvalue_6))
        (set `self.Offset Z` (+ (/ (* (`self.Rows`) _returnvalue_4) 2.0) _returnvalue_6))
        (for _index (range (`self.Rows`))
          (for _index_2 (range (`self.Columns`))
            (bind _returnvalue_8 (+ _returnvalue_y (* (+ _index_2 1) _scaler) (`self.Offset Y`)))
            (bind _returnvalue_9 (+ _returnvalue_z (* (+ _index 1) (* _scaler -1.0)) (`self.Offset Z`)))
            (`KismetArrayLibrary.Array_Add` (`self.Grid Locations`) (`KismetMathLibrary.MakeTransform` (+ (`KismetMathLibrary.GreaterGreater_VectorRotator` (- (`KismetMathLibrary.MakeVector` (+ _returnvalue_x (`self.Scaler`)) _returnvalue_8 _returnvalue_9) _returnvalue_2) _returnvalue) _returnvalue_2) _returnvalue _returnvalue_5))
            (`KismetArrayLibrary.Array_Add` (`self.Grid Locations Forward`) (`KismetMathLibrary.MakeTransform` (+ (`KismetMathLibrary.GreaterGreater_VectorRotator` (- (`KismetMathLibrary.MakeVector` _returnvalue_x_2 _returnvalue_8 _returnvalue_9) _returnvalue_2) _returnvalue) _returnvalue_2) _returnvalue _returnvalue_5))))
        (`self.Spawn Cubes`)))))

(event `self.ReceiveBeginPlay`
  (bind _returnvalue (* (`KismetMathLibrary.RandomFloat`) 10.0))
  (`self.UpdateState`)
  ;[1 1 1] Cube Stuff
  (`MeshComponent.SetScalarParameterValueOnMaterials` (`self.sponny`) "Seed" _returnvalue)
  (`MeshComponent.SetScalarParameterValueOnMaterials` (`self.spanny`) "Seed" _returnvalue)
  (`MeshComponent.SetScalarParameterValueOnMaterials` (`self.spinny`) "Seed" _returnvalue))

(event `Spawn Cubes`
  (bind (_returnvalue_location _returnvalue_rotation _returnvalue_scale) (`KismetMathLibrary.BreakTransform` (`SceneComponent.K2_GetComponentToWorld` (`self.Root`))))
  ;[1 1 1] Cubes
  (for (_array_element _array_index) (`self.Grid Objects`)
    (set `self.Root Spwn Transform` (`KismetMathLibrary.MakeTransform` _returnvalue_location (`KismetMathLibrary.RandomRotator` false) _returnvalue_scale))
    (switch `string` _array_element
      (:`BP_BackBord_Brick`
        (bind _output (`|GetArrayItem` (`self.Grid Locations`) _array_index))
        (bind _returnvalue (`|SpawnActorFromClass` "/Game/PathWays/Blueprints/Bricks/BP_BackBord_Brick.BP_BackBord_Brick_C" (`self.Root Spwn Transform`) "AlwaysSpawn" "MultiplyWithRoot" null _output null))
        (`KismetArrayLibrary.Array_Add` (`self.Spawned Cube Stuff`) _returnvalue))
      (:`BP_Blocking_Brick`
        (bind _returnvalue_2 (`|SpawnActorFromClass` "/Game/PathWays/Blueprints/Bricks/BP_Blocking_Brick.BP_Blocking_Brick_C" (`self.Root Spwn Transform`) "AlwaysSpawn" "MultiplyWithRoot" null _output null))
        (`KismetArrayLibrary.Array_Add` (`self.Spawned Cube Stuff`) _returnvalue_2)
        (bind _output_2 (`|GetArrayItem` (`self.Grid Locations Forward`) _array_index))
        (bind _returnvalue_3 (`|SpawnActorFromClass` "/Game/PathWays/Blueprints/Bricks/BP_Blocking_Brick.BP_Blocking_Brick_C" (`self.Root Spwn Transform`) "AlwaysSpawn" "MultiplyWithRoot" null _output_2 null))
        (`KismetArrayLibrary.Array_Add` (`self.Spawned Cube Stuff`) _returnvalue_3))
      (:`BP_Border_Brick`
        (bind _returnvalue_4 (`|SpawnActorFromClass` "/Game/PathWays/Blueprints/Bricks/BP_Border_Brick.BP_Border_Brick_C" (`self.Root Spwn Transform`) "AlwaysSpawn" "MultiplyWithRoot" null _output null))
        (`KismetArrayLibrary.Array_Add` (`self.Spawned Cube Stuff`) _returnvalue_4)
        (bind _returnvalue_5 (`|SpawnActorFromClass` "/Game/PathWays/Blueprints/Bricks/BP_Border_Brick.BP_Border_Brick_C" (`self.Root Spwn Transform`) "AlwaysSpawn" "MultiplyWithRoot" null _output_2 null))
        (`KismetArrayLibrary.Array_Add` (`self.Spawned Cube Stuff`) _returnvalue_5))
      (:`BP_OrangeCL_Brick`
        ;;[0.8494 0.3222 1] ColorLines
        (bind _returnvalue_6 (`|SpawnActorFromClass` "/Game/PathWays/Blueprints/Bricks/BP_BackBord_Brick.BP_BackBord_Brick_C" (`self.Root Spwn Transform`) "AlwaysSpawn" "MultiplyWithRoot" null _output null))
        (`KismetArrayLibrary.Array_Add` (`self.Spawned Cube Stuff`) _returnvalue_6)
        (bind _returnvalue_7 (`|SpawnActorFromClass` "/Game/PathWays/Blueprints/Bricks/BP_OrangeCL_Brick.BP_OrangeCL_Brick_C" (`self.Root Spwn Transform`) "AlwaysSpawn" "MultiplyWithRoot" null _output_2 null))
        (`KismetArrayLibrary.Array_Add` (`self.Spawned Cube Stuff`) _returnvalue_7))
      (:`BP_GreenCL_Brick`
        (bind _returnvalue_8 (`|SpawnActorFromClass` "/Game/PathWays/Blueprints/Bricks/BP_BackBord_Brick.BP_BackBord_Brick_C" (`self.Root Spwn Transform`) "AlwaysSpawn" "MultiplyWithRoot" null _output null))
        (`KismetArrayLibrary.Array_Add` (`self.Spawned Cube Stuff`) _returnvalue_8)
        (bind _returnvalue_9 (`|SpawnActorFromClass` "/Game/PathWays/Blueprints/Bricks/BP_GreenCL_Brick.BP_GreenCL_Brick_C" (`self.Root Spwn Transform`) "AlwaysSpawn" "MultiplyWithRoot" null _output_2 null))
        (`KismetArrayLibrary.Array_Add` (`self.Spawned Cube Stuff`) _returnvalue_9))
      (:`BP_OrangeGoal_Brick`
        (bind _returnvalue_10 (`|SpawnActorFromClass` "/Game/PathWays/Blueprints/Bricks/BP_OrangeGoal_Brick.BP_OrangeGoal_Brick_C" (`self.Root Spwn Transform`) "AlwaysSpawn" "MultiplyWithRoot" null _output null))
        (`KismetArrayLibrary.Array_Add` (`self.Spawned Cube Stuff`) _returnvalue_10))
      (:`BP_GreenGoal_Brick`
        (bind _returnvalue_11 (`|SpawnActorFromClass` "/Game/PathWays/Blueprints/Bricks/BP_GreenGoal_Brick.BP_GreenGoal_Brick_C" (`self.Root Spwn Transform`) "AlwaysSpawn" "MultiplyWithRoot" null _output null))
        (`KismetArrayLibrary.Array_Add` (`self.Spawned Cube Stuff`) _returnvalue_11))))
  (bind _returnvalue_12 (`GameplayStatics.GetActorOfClass` "/Game/PathWays/Blueprints/Bricks/BP_ColorLine_Brick.BP_ColorLine_Brick_C"))
  (`Controller.Possess` (`GameplayStatics.GetPlayerController` 0) _returnvalue_12))

(event `self.ReceiveTick`
  (params (DeltaSeconds :type "Float (single-precision)"))
  (bind _speed_1 (`self.Speed 1`))
  (bind _speed_3 (`self.Speed 3`))
  (bind _speed_2 (`self.Speed 2`))
  ;[1 1 1] Cube Stuff
  (`SceneComponent.K2_AddLocalRotation` (`self.spinny`) (`KismetMathLibrary.MakeRotator` _speed_1 _speed_2 _speed_3) false false)
  (`SceneComponent.K2_AddLocalRotation` (`self.sponny`) (`KismetMathLibrary.MakeRotator` _speed_3 _speed_1 _speed_2) false false)
  (`SceneComponent.K2_AddLocalRotation` (`self.spanny`) (`KismetMathLibrary.MakeRotator` _speed_2 _speed_3 _speed_1) false false))

(fn `UpdateState`
  (locals (`Color I1` :type "Color Structure" :default (struct :`B` 188 :`G` 255 :`R` 255)) (`Color I2` :type "Color Structure" :default (struct :`B` 255 :`G` 251 :`R` 188)) (`Color I3` :type "Color Structure" :default (struct :`B` 247 :`G` 188 :`R` 255)) (`Color T1` :type "Color Structure") (`Color T2` :type "Color Structure") (`Color T3` :type "Color Structure") (`Color U1` :type "Color Structure" :default (struct :`R` 255)) (`Color U2` :type "Color Structure" :default (struct :`B` 194 :`R` 255)) (`Color U3` :type "Color Structure" :default (struct :`G` 184 :`R` 255)) (`Color S1` :type "Color Structure" :default (struct :`B` 255 :`G` 255)) (`Color S2` :type "Color Structure" :default (struct :`G` 255)) (`Color S3` :type "Color Structure" :default (struct :`B` 188 :`G` 188)))
  (switch `/Game/PathWays/Blueprints/E_Podium_State` (`self.State`)
    (:`NewEnumerator0`
      ;[1 1 1] Colors
      (set `local.Color T1` (`local.Color I1`))
      (set `local.Color T2` (`local.Color I2`))
      (set `local.Color T3` (`local.Color I3`))
      (`|ExecutionSequence`
        (:`then_0`
          _)))
    (:`NewEnumerator1`
      (set `local.Color T1` (`local.Color U1`))
      (set `local.Color T2` (`local.Color U2`))
      (set `local.Color T3` (`local.Color U3`))
      (`|ExecutionSequence`
        (:`then_0`
          _)))
    (:`NewEnumerator2`
      (set `local.Color T1` (`local.Color S1`))
      (set `local.Color T2` (`local.Color S2`))
      (set `local.Color T3` (`local.Color S3`))
      (`|ExecutionSequence`
        (:`then_0`
          _))))
  ;[1 1 1] COLORS
  (bind _returnvalue (`PrimitiveComponent.CreateDynamicMaterialInstance` (`self.sponny`) 0 null "None"))
  (`MaterialInstanceDynamic.SetVectorParameterValue` _returnvalue "Color 1" (`KismetMathLibrary.Conv_ColorToLinearColor` (`local.Color T1`)))
  (`MaterialInstanceDynamic.SetVectorParameterValue` _returnvalue "Color 2" (`KismetMathLibrary.Conv_ColorToLinearColor` (`local.Color T2`)))
  (`MaterialInstanceDynamic.SetVectorParameterValue` _returnvalue "Color 3" (`KismetMathLibrary.Conv_ColorToLinearColor` (`local.Color T3`)))
  (bind _returnvalue_2 (`PrimitiveComponent.CreateDynamicMaterialInstance` (`self.spanny`) 0 null "None"))
  (`MaterialInstanceDynamic.SetVectorParameterValue` _returnvalue_2 "Color 1" (`KismetMathLibrary.Conv_ColorToLinearColor` (`local.Color T1`)))
  (`MaterialInstanceDynamic.SetVectorParameterValue` _returnvalue_2 "Color 2" (`KismetMathLibrary.Conv_ColorToLinearColor` (`local.Color T2`)))
  (`MaterialInstanceDynamic.SetVectorParameterValue` _returnvalue_2 "Color 3" (`KismetMathLibrary.Conv_ColorToLinearColor` (`local.Color T3`)))
  (bind _returnvalue_3 (`PrimitiveComponent.CreateDynamicMaterialInstance` (`self.spinny`) 0 null "None"))
  (`MaterialInstanceDynamic.SetVectorParameterValue` _returnvalue_3 "Color 1" (`KismetMathLibrary.Conv_ColorToLinearColor` (`local.Color T1`)))
  (`MaterialInstanceDynamic.SetVectorParameterValue` _returnvalue_3 "Color 2" (`KismetMathLibrary.Conv_ColorToLinearColor` (`local.Color T2`)))
  (`MaterialInstanceDynamic.SetVectorParameterValue` _returnvalue_3 "Color 3" (`KismetMathLibrary.Conv_ColorToLinearColor` (`local.Color T3`))))

(fn `UserConstructionScript`)